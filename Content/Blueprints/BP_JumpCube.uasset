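; A cube platform that moves back and forth along DestTransform each time the pawn standing on it jumps.
; OnPawnon and OnPawnOff swap the grid material and bind or unbind Toggle to the pawn's jump event, and Toggle flip-flops a Timeline between play and reverse.
; Each update applies only the delta from the previous lerped transform, cached in DummyCube, to the actor's current transform.
; Reset re-triggers the flip-flop to reverse a cube that was toggled forward.
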(event `/Game/Blueprints/Interfaces/BI_Floor.OnPawnOn`
  (params (Pawn :type "Pawn Object Reference"))
  (`PrimitiveComponent.SetMaterial` (`self.Cube`) 0 "/Game/DragMe/GridMaterials/MI_Grid_G.MI_Grid_G")
  (bind _asbp_pawn (cast `/Game/Blueprints/BP_Pawn` Pawn))
  (add `/Game/Blueprints/BP_Pawn.OnPawnJumped` _asbp_pawn (delegate `Toggle`)))

(event `Toggle`
  (bind _isa (`/Engine/EditorBlueprintResources/StandardMacros.FlipFlop` :!label _label)
    (:`A`
      ;[1 1 1] Cubeの上下動
      (bind (_direction _alpha) (`Timeline|Timeline` :!label _label_2)
        (:`Update`
          (bind _returnvalue (`KismetMathLibrary.TLerp` (`self.Identity`) (`self.DestTransform`) _alpha))
          (`self.K2_SetActorTransform` (`KismetMathLibrary.ComposeTransforms` (`KismetMathLibrary.ComposeTransforms` _returnvalue (`KismetMathLibrary.InvertTransform` (`self.DummyCube`))) (`self.GetTransform`)))
          (set `self.DummyCube` _returnvalue))))
    (:`B`
      (goto _label_2 :!via `Reverse`))))

(event `Reset`
  (if (stale `Toggle` _isa)
    (goto _label)))

(event `/Game/Blueprints/Interfaces/BI_Floor.OnPawnOff`
  (params (Pawn :type "Pawn Object Reference"))
  (`PrimitiveComponent.SetMaterial` (`self.Cube`) 0 "/Game/DragMe/GridMaterials/MI_Grid_Y.MI_Grid_Y")
  (bind _asbp_pawn (cast `/Game/Blueprints/BP_Pawn` Pawn))
  (remove `/Game/Blueprints/BP_Pawn.OnPawnJumped` _asbp_pawn (delegate `Toggle`)))

(fn `UserConstructionScript`)