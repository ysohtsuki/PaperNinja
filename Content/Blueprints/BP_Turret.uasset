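; Turret actor that fires a burst of BP_Bullet projectiles when its Sensor component detects something, polled every Tick.
; A DoOnce-gated timeline spins the barrel through RotatingMovement, and its Fire event track uses a FlipFlop to alternately start and clear a looping FireRate-based timer.
; Each shot spawns a bullet at the Muzzle socket with random yaw spread and draws debug text.
; The DoOnce resets when the timeline finishes, allowing the next burst.
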(event `self.ReceiveBeginPlay`
  (`MovementComponent.SetUpdatedComponent` (`self.RotatingMovement`) (`self.Barrel`)))

(event `StartFire`
  (bind _returnvalue (`KismetMathLibrary.SafeDivide` 1.0 (`self.FireRate`)))
  (`/Engine/EditorBlueprintResources/StandardMacros.DoOnce` false :!label _label
    (:`Completed`
      (bind (_direction _muzzlerolling _bulletcolor) (`Timeline|FireControlTL` :!via `PlayFromStart`)
        (:`Update`
          (set `RotatingMovementComponent.RotationRate` (`KismetMathLibrary.MakeRotator` _muzzlerolling) (`self.RotatingMovement`)))
        (:`Finished`
          (goto _label :!via `Reset`))
        (:`Fire`
          (`/Engine/EditorBlueprintResources/StandardMacros.FlipFlop`
            (:`A`
              (bind _returnvalue_2 (`KismetSystemLibrary.K2_SetTimerDelegate` (delegate `Fire`) _returnvalue true (* _returnvalue -1.0))))
            (:`B`
              (`KismetSystemLibrary.K2_ClearAndInvalidateTimerHandle` _returnvalue_2))))))))

(event `Fire`
  (`KismetSystemLibrary.DrawDebugString` (0.0 0.0 0.0) "Fire!" self (stale `StartFire` _bulletcolor) 0.2) ; Fireのデバッグ表示
  ;[1 1 1] 弾丸のスポーン
  (`|SpawnActorFromClass` "/Game/Blueprints/BP_Bullet.BP_Bullet_C" (`KismetMathLibrary.ComposeTransforms` (`self.GetLocalSpread`) (`self.GetMuzzleTransform`)) "Undefined" "OverrideRootScale" null 600.0 0.2 null))

(event `self.ReceiveTick`
  (params (DeltaSeconds :type "Float (single-precision)"))
  ;[1 1 1] センサーコンポーネントをチェックし、反応があれば射撃を開始する
  (bind (_outactors _returnvalue) (`/Game/Blueprints/Components/AC_Sensor.CheckSensor` (`self.Sensor`)))
  (if _returnvalue
    (`self.StartFire`)))

(fn `GetLocalSpread`
  (returns (ReturnValue :type "Transform Structure"))
  ;[1 1 1] 銃口のブレのトランスフォームを作成
  (return (`KismetMathLibrary.MakeTransform` (0.0 0.0 0.0) (`KismetMathLibrary.MakeRotator` 0.0 0.0 (`KismetMathLibrary.RandomFloatInRange` -10.0 10.0)))))

(fn `GetMuzzleTransform`
  (returns (ReturnValue :type "Transform Structure"))
  (return (`SceneComponent.GetSocketTransform` (`self.StaticMeshComponent`) "Muzzle" "RTS_World")))

(fn `UserConstructionScript`)