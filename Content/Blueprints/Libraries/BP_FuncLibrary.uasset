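; BP_FuncLibrary is a Blueprint function library of small math and gameplay helpers.
; CalcRay turns an origin, direction and length into start and end points.
; IsPlayerPawn returns true only for a Pawn controlled by a PlayerController.
; SineCurve evaluates a sine wave from amplitude, period, time and phase, converting period to angular frequency with a safe divide and feeding a math expression.
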(fn CalcRay
  (params (Origin :type Vector) (Direction :type Vector) (Length :type Float%20%28double-precision%29))
  (return Origin (+ Origin (* Direction Length))))

(fn IsPlayerPawn
  (params (Actor :type Actor%20Object%20Reference))
  (bind _aspawn (Utilities|Casting|CastToPawn Actor)
    (:then
      (Utilities|Casting|CastToPlayerController (Pawn|GetController _aspawn)
        (:then
          (return true))
        (:CastFailed
          _)))
    (:CastFailed
      _))
  (return false))

(fn SineCurve
  (params (Amplitude :type Float%20%28double-precision%29) (Period :type Float%20%28double-precision%29) (Time :type Float%20%28double-precision%29) (Phase :type Float%20%28double-precision%29))
  ;[1 1 1] A*sin((2pi/T)*t+θ)
  (return (|(A*(sin(((w*t)+theta)))) Amplitude (Math|Float|SafeDivide (Math|Float|MultiplybyPi 2.0) Period) Time Phase)))