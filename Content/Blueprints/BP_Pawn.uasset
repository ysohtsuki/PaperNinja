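; Player character Blueprint with camera-relative movement, look, jump and sprint, plus an optional weapon mesh attached to a hand socket at construction.
; Tick compares the current floor actor to the last one and notifies both through the BI_Floor interface as the pawn steps off and on.
; Any damage kills it once, triggering a launched ragdoll and timed lifespan, while hits damage the other actor.
; Jumps are delayed when nearly stationary and also notify floor logic.
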(event `self.ReceiveBeginPlay`)

(event `self.ReceiveTick`
  (params (DeltaSeconds :type "Float (single-precision)"))
  (bind _floor (`self.GetCurrentFloor`))
  ;[1 1 1] 床チェックと通知
  (if (!= (`self.GetCurrentFloor`) (`self.LastFloor`))
    (`|ExecutionSequence`
      (:`then_0`
        (bind _asbi_floor (cast `/Game/Blueprints/Interfaces/BI_Floor` (`self.LastFloor`)))
        (`/Game/Blueprints/Interfaces/BI_Floor.OnPawnOff` _asbi_floor self))
      (:`then_1`
        (bind _asbi_floor_2 (cast `/Game/Blueprints/Interfaces/BI_Floor` _floor))
        (`/Game/Blueprints/Interfaces/BI_Floor.OnPawnOn` _asbi_floor_2 self))
      (:`then_2`
        (set `self.LastFloor` _floor)))))

(event `self.ReceiveAnyDamage`
  (params (Damage :type "Float (single-precision)") (DamageType :type "DamageType Object Reference") (InstigatedBy :type "Controller Object Reference") (DamageCauser :type "Actor Object Reference"))
  (bind _mesh (`self.Mesh`))
  (`/Engine/EditorBlueprintResources/StandardMacros.DoOnce` false
    (:`Completed`
      (`KismetSystemLibrary.PrintString` "Died!")
      (`CharacterMovementComponent.DisableMovement` (`self.CharacterMovement`)) ; キャラクターを動けなくする
      (`self.SetLifeSpan` 5.0) ; 5.0秒の寿命をつける
      ;[1 1 1] ラグドール処理
      (`PrimitiveComponent.SetCollisionProfileName` _mesh "Ragdoll" true)
      (`SkeletalMeshComponent.SetAllBodiesSimulatePhysics` _mesh true)
      (`SkeletalMeshComponent.AddImpulseToAllBodiesBelow` _mesh (0.0 0.0 300.0) "None" true true)
      (`PrimitiveComponent.SetCollisionProfileName` (`self.CapsuleComponent`) "Spectator" true))))

(event `self.ReceiveHit`
  (params (MyComp :type "PrimitiveComponent Object Reference") (Other :type "Actor Object Reference") (OtherComp :type "PrimitiveComponent Object Reference") (bSelfMoved :type Boolean) (HitLocation :type "Vector Structure") (HitNormal :type "Vector Structure") (NormalImpulse :type "Vector Structure") (Hit :type "HitResult Structure (by ref)"))
  ;[1 1 1] Hit相手にダメージを適用
  (`GameplayStatics.ApplyDamage` Other 1.0 null self))

(event `self.OnJumped`
  ;[1 1 1] ジャンプ開始通知
  (`self.OnPawnJumped`))

(event `EnhancedInput|/Game/Inputs/IA_Jump`
  (params (ActionValue :type Boolean) (ElapsedSeconds :type "Float (double-precision)") (TriggeredSeconds :type "Float (double-precision)") (InputAction :type "InputAction Object Reference" :default "/Game/Inputs/IA_Jump.IA_Jump"))
  (:`Triggered`
    (if (`self.CanJump`)
      (if (not (>= (`KismetMathLibrary.VSizeXY` (`self.GetVelocity`)) 10.0))
        (`KismetSystemLibrary.Delay` 0.3))
      (`self.Jump`))))

(event `EnhancedInput|/Game/Inputs/IA_Sprint`
  (params (ActionValue :type Boolean) (ElapsedSeconds :type "Float (double-precision)") (TriggeredSeconds :type "Float (double-precision)") (InputAction :type "InputAction Object Reference" :default "/Game/Inputs/IA_Sprint.IA_Sprint"))
  (:`Triggered`
    (`self.BeginSprint`))
  (:`Completed`
    (`self.EndSprint`)))

(event `EnhancedInput|/Game/Inputs/IA_ForceKill`
  (params (ActionValue :type Boolean) (ElapsedSeconds :type "Float (double-precision)") (TriggeredSeconds :type "Float (double-precision)") (InputAction :type "InputAction Object Reference" :default "/Game/Inputs/IA_ForceKill.IA_ForceKill"))
  ;[1 1 1] フォースキル
  (:`Triggered`
    (`GameplayStatics.ApplyDamage` self 1.0)))

(event `EnhancedInput|/Game/Inputs/IA_Look`
  (params (ActionValue :type "Vector2D Structure") (ElapsedSeconds :type "Float (double-precision)") (TriggeredSeconds :type "Float (double-precision)") (InputAction :type "InputAction Object Reference" :default "/Game/Inputs/IA_Look.IA_Look"))
  (bind (_x _y) (`KismetMathLibrary.BreakVector2D` ActionValue))
  ;[1 1 1] カメラ制御
  (:`Triggered`
    (`self.AddControllerYawInput` _x)
    (`self.AddControllerPitchInput` _y)))

(event `EnhancedInput|/Game/Inputs/IA_Move`
  (params (ActionValue :type "Vector2D Structure") (ElapsedSeconds :type "Float (double-precision)") (TriggeredSeconds :type "Float (double-precision)") (InputAction :type "InputAction Object Reference" :default "/Game/Inputs/IA_Move.IA_Move"))
  (bind (_x _y) (`KismetMathLibrary.BreakVector2D` ActionValue))
  ;[1 1 1] 移動
  (:`Triggered`
    (`self.AddMovementInput` (`SceneComponent.GetRightVector` (`self.Camera`)) _x) ; 左右移動
    (`self.AddMovementInput` (`KismetMathLibrary.Cross_VectorVector` (`SceneComponent.GetRightVector` (`self.Camera`)) (`KismetMathLibrary.Vector_Up`)) _y) ; 前後移動
  ))

(fn `BeginSprint`
  (returns (Succeed :type Boolean))
  (locals (AccelCurve :type "CurveFloat Object Reference" :default null))
  (if (`self.IsSprinting`)
    (return false)
    (else
      (set `CharacterMovementComponent.MaxWalkSpeed` 200.0 (`self.CharacterMovement`))
      (set `self.IsSprinting` true)
      (return true))))

(fn `EndSprint`
  (returns (Succeed :type Boolean))
  (if (`self.IsSprinting`)
    (set `CharacterMovementComponent.MaxWalkSpeed` 75.0 (`self.CharacterMovement`))
    (set `self.IsSprinting` false)
    (return true)
    (else
      (return false))))

(fn `GetCurrentFloor`
  (returns (Floor :type "Actor Object Reference"))
  ;[1 1 1] 現在踏んでいる床のアクタ参照を返す
  (return (`.HitActor` (`GameplayStatics.BreakHitResult` (`.HitResult` (break `FindFloorResult` (`CharacterMovementComponent.CurrentFloor` (`self.CharacterMovement`))))))))

(fn `GetIsSprinting`
  (returns (ReturnValue :type Boolean))
  (return (`self.IsSprinting`)))

(fn `UserConstructionScript`
  (locals (WeaponMesh :type "StaticMeshComponent Object Reference"))
  ;[1 1 1] 武器の設定
  (`/Engine/EditorBlueprintResources/StandardMacros.IsValid` (`self.WeaponMeshAsset`)
    (:`Is Valid`
      (bind _returnvalue (`AddComponent|NODE_AddStaticMeshComponent-1` :`bManualAttachment` true))
      (bind _output_get (set `local.WeaponMesh` _returnvalue))
      (`StaticMeshComponent.SetStaticMesh` _output_get (`self.WeaponMeshAsset`))
      (`SceneComponent.K2_AttachToComponent` (`local.WeaponMesh`) (`self.Mesh`) "weapon_r" "SnapToTarget" "SnapToTarget" "SnapToTarget" true))))