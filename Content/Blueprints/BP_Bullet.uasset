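; Physics-driven bullet actor that launches along its forward vector and damages the first actor it hits.
; BeginPlay applies a velocity-change impulse, and Tick adds upward acceleration blended by GravityScale to offset gravity, acting as lift.
; The first hit applies damage, stops Tick so the lift ends, and sets the mesh to ignore the Pawn channel so the spent bullet no longer hits pawns.
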(event `self.ReceiveBeginPlay`
  (`PrimitiveComponent.AddImpulse` (`self.StaticMeshComponent`) (* (`self.GetActorForwardVector`) (`self.BulletInitialSpeed`)) "None" true))

(event `self.ReceiveTick`
  (params (DeltaSeconds :type "Float (single-precision)"))
  ;[1 1 1] 揚力を効かせる
  (`PrimitiveComponent.AddForce` (`self.StaticMeshComponent`) (`KismetMathLibrary.VLerp` (0.0 0.0 980.0) (0.0 0.0 0.0) (`self.GravityScale`)) "None" true))

(event `self.ReceiveHit`
  (params (MyComp :type "PrimitiveComponent Object Reference") (Other :type "Actor Object Reference") (OtherComp :type "PrimitiveComponent Object Reference") (bSelfMoved :type Boolean) (HitLocation :type "Vector Structure") (HitNormal :type "Vector Structure") (NormalImpulse :type "Vector Structure") (Hit :type "HitResult Structure (by ref)"))
  ;[1 1 1] Hit相手にダメージを適用
  (`/Engine/EditorBlueprintResources/StandardMacros.DoOnce` false
    (:`Completed`
      (`GameplayStatics.ApplyDamage` Other 1.0 null self)
      (`self.SetActorTickEnabled` false)
      ;[1 1 1] 対ポーンヒットの無効化
      (`PrimitiveComponent.SetCollisionResponseToChannel` (`self.StaticMeshComponent`) "ECC_Pawn" "ECR_Ignore"))))

(fn `UserConstructionScript`)