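; AC_Sensor is a sight sensor component that detects actors inside a view cone along its forward vector, defined by sight length and angle.
; CheckSensor gathers candidates with a box trace sized to the cone, draws a debug cone, and returns visible actors plus a found flag.
; CanSeeActor filters each candidate by a dot-product angle test before running a line trace to confirm an unobstructed view.
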(fn `CanSeeActor`
  (params (TargetActor :type "Actor Object Reference"))
  (returns (ReturnValue :type Boolean))
  (bind _returnvalue (`Actor.K2_GetActorLocation` TargetActor))
  ;[1 1 1] ライントレースを飛ばす前に角度チェックを行う
  (if (`self.IsInSight` _returnvalue)
    ;[1 1 1] ターゲットのアクタに視線ライントレースが通るかを判定
    (bind _outhit (`KismetSystemLibrary.LineTraceSingle` :`Start` (`self.K2_GetComponentLocation`) :`End` _returnvalue :`TraceChannel` "TraceTypeQuery3" :`DrawDebugType` "ForOneFrame"))
    (return (== TargetActor (`.HitActor` (`GameplayStatics.BreakHitResult` _outhit))))
    (else
      (return false))))

(fn `CheckSensor`
  (returns (OutActors :type "Array of Actor Object Reference") (ReturnValue :type Boolean))
  (locals (ReturnActors :type "Array of Actor Object Reference"))
  (bind _returnactors (`local.ReturnActors`))
  (bind _location (.location (`self.K2_GetComponentToWorld`)))
  (bind _rotation (.rotation (`self.K2_GetComponentToWorld`)))
  (bind _returnvalue (* (`self.SightAngle`) 0.5))
  (bind _returnvalue_2 (`KismetMathLibrary.GetForwardVector` _rotation))
  (bind (_start _end) (`/Game/Blueprints/Libraries/BP_FuncLibrary.CalcRay` _location _returnvalue_2 (`self.SightLength`)))
  (bind _returnvalue_3 (* (`self.SightLength`) (`KismetMathLibrary.DegTan` (* (`self.SightAngle`) 0.5))))
  ;[1 1 1] コメント
  (bind _outhits (`KismetSystemLibrary.BoxTraceMulti` _start _end (`KismetMathLibrary.MakeVector` 1.0 _returnvalue_3 _returnvalue_3) _rotation "TraceTypeQuery4"))
  (`KismetSystemLibrary.DrawDebugConeInDegrees` _location _returnvalue_2 (`self.SightLength`) _returnvalue _returnvalue 6 (struct :`R` 0.886643 :`B` 1.0 :`A` 1.0))
  ;;[1 1 1] 視界に入ったアクタをすべて配列に入れて返す
  (for _array_element _outhits
    (bind (_bblockinghit _binitialoverlap _time _distance _location_2 _impactpoint _normal _impactnormal _physmat _hitactor) (`GameplayStatics.BreakHitResult` _array_element))
    (bind _returnvalue_4 (`self.CanSeeActor` _hitactor))
    (if _returnvalue_4
      (`KismetArrayLibrary.Array_Add` (`local.ReturnActors`) _hitactor)))
  (return _returnactors (`KismetArrayLibrary.Array_IsNotEmpty` _returnactors)))

(fn `IsInSight`
  (params (TargetLocation :type "Vector Structure"))
  (returns (ReturnValue :type Boolean))
  ;[1 1 1] TargetLocationがSightAngleの内側かどうか調べる
  (return (<= (`KismetMathLibrary.DegAcos` (`KismetMathLibrary.Dot_VectorVector` (`KismetMathLibrary.GetDirectionUnitVector` (`self.K2_GetComponentLocation`) TargetLocation) (`self.GetForwardVector`))) (* (`self.SightAngle`) 0.5))))