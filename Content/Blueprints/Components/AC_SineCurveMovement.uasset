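; Actor component that moves its owning actor back and forth around its starting position along sine waves.
; BeginPlay records the owner's location as the origin.
; Each tick evaluates a SineCurve per axis from game time, using vector Amplitude, Period and Phase settings, and adds the result to that origin.
; The location is set directly without sweeping, so movement ignores blocking collision.
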(event `self.ReceiveBeginPlay`
  ;[1 1 1] 初期位置を記録
  (set `self.Initial Location` (`Actor.K2_GetActorLocation` (`self.GetOwner`))))

(event `self.ReceiveTick`
  (params (DeltaSeconds :type "Float (single-precision)"))
  (bind _returnvalue (`KismetSystemLibrary.GetGameTimeInSeconds`))
  (bind (_amplitude_x _amplitude_y _amplitude_z) (`KismetMathLibrary.BreakVector` (`self.Amplitude`)))
  (bind (_period_x _period_y _period_z) (`KismetMathLibrary.BreakVector` (`self.Period`)))
  (bind (_phase_x _phase_y _phase_z) (`KismetMathLibrary.BreakVector` (`self.Phase`)))
  ;[1 1 1] 正弦波で動かす
  (`Actor.K2_SetActorLocation` (`self.GetOwner`) (+ (`KismetMathLibrary.MakeVector` (`/Game/Blueprints/Libraries/BP_FuncLibrary.SineCurve` _amplitude_x _period_x _returnvalue _phase_x) (`/Game/Blueprints/Libraries/BP_FuncLibrary.SineCurve` _amplitude_y _period_y _returnvalue _phase_y) (`/Game/Blueprints/Libraries/BP_FuncLibrary.SineCurve` _amplitude_z _period_z _returnvalue _phase_z)) (`self.Initial Location`)) false false))